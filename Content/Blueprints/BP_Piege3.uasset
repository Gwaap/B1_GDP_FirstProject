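; BP_Piege3 is a trap actor that tips over by pitching 90 degrees after the third-person character enters its box.
; BeginPlay stores the starting rotation and derives the target rotation from it.
; The overlap waits through a short delay, then starts a looping timer on OpenTrap.
; Each tick of that timer eases the actor toward the target with a small-alpha rotator lerp, clearing itself once nearly there; nothing resets the trap.
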(event `self.ReceiveBeginPlay`
  (bind _output_get (set `self.DefaultRotation` (`self.K2_GetActorRotation`)))
  (set `self.FinalRotation` (`KismetMathLibrary.MakeRotator` (.roll _output_get) (+ (.pitch _output_get) 90.0) (.yaw _output_get))))

(event `self.Box.OnComponentBeginOverlap`
  (params (OverlappedComponent :type "PrimitiveComponent Object Reference") (OtherActor :type "Actor Object Reference") (OtherComp :type "PrimitiveComponent Object Reference") (OtherBodyIndex :type Integer) (bFromSweep :type Boolean) (SweepResult :type "HitResult Structure (by ref)"))
  (cast `/Game/ThirdPersonBP/Blueprints/ThirdPersonCharacter` OtherActor)
  (`KismetSystemLibrary.Delay` 2.0)
  (`KismetSystemLibrary.K2_SetTimer` null "OpenTrap" 0.01 true))

(fn `OpenTrap`
  (bind _finalrotation (`self.FinalRotation`))
  (bind _returnvalue (`KismetMathLibrary.RLerp` (`self.K2_GetActorRotation`) _finalrotation 0.01))
  (`self.K2_SetActorRotation` _returnvalue)
  (if (== _returnvalue _finalrotation :`ErrorTolerance` 2.0)
    (`KismetSystemLibrary.K2_ClearTimer` null "OpenTrap")))

(fn `UserConstructionScript`)