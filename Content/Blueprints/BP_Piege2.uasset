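; BP_Piege2 is a self-resetting trap with a cube that drops under physics after the third-person character enters its trigger box.
; The overlap starts a two-second delay before physics simulation is enabled on the cube.
; Five seconds later it spawns a fresh copy of itself at the transform saved on BeginPlay and destroys itself, resetting the trap by replacement.
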(event `self.ReceiveBeginPlay`
  (set `self.DefaultSpawn` (`self.GetTransform`)))

(event `self.Box.OnComponentBeginOverlap`
  (params (OverlappedComponent :type "PrimitiveComponent Object Reference") (OtherActor :type "Actor Object Reference") (OtherComp :type "PrimitiveComponent Object Reference") (OtherBodyIndex :type Integer) (bFromSweep :type Boolean) (SweepResult :type "HitResult Structure (by ref)"))
  (cast `/Game/ThirdPersonBP/Blueprints/ThirdPersonCharacter` OtherActor)
  (`KismetSystemLibrary.Delay` 2.0)
  (`PrimitiveComponent.SetSimulatePhysics` (`self.Cube`) true)
  (`KismetSystemLibrary.Delay` 5.0)
  (`|SpawnActorFromClass` "BP_Piege2_C" (`self.DefaultSpawn`) "Undefined" "OverrideRootScale" null null)
  (`self.K2_DestroyActor`))

(fn `UserConstructionScript`)